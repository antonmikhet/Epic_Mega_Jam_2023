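; BP_Antenna_Second is a sequence actor for an antenna that turns to aim and then fires a beam.
; AntennaAim uses a timeline to lerp the Antenna's relative rotation from its current value to AntennaRotation, then calls BeamOn when finished.
; BeamOn plays a 2D sound and uses a second timeline to stretch the Cylinder mesh along Z into a long beam.
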(event `BeamOn`
  (bind _startbeamtransform (`self.StartBeamTransform`))
  (bind (_startbeamtransform_location _startbeamtransform_rotation _startbeamtransform_scale) (`KismetMathLibrary.BreakTransform` (`self.StartBeamTransform`)))
  (set `self.StartBeamTransform` (`SceneComponent.GetRelativeTransform` (`self.Cylinder`)))
  (`GameplayStatics.PlaySound2D` "/Game/EpicMegaJam2023/Core/Audio/Metasounds/MS_ANtenna.MS_ANtenna" 1.0 1.0 0.0 null null)
  (bind (_direction _newtrack_0) (`Timeline|BeamTimeline`)
    (:`Update`
      (`SceneComponent.K2_SetRelativeTransform` (`self.Cylinder`) (`KismetMathLibrary.MakeTransform` _startbeamtransform_location _startbeamtransform_rotation (`KismetMathLibrary.VLerp` _startbeamtransform_scale (`KismetMathLibrary.MakeVector` (.x (.scale _startbeamtransform)) (.y (.scale _startbeamtransform)) 200.0) _newtrack_0)) false false))))

(event `AntennaAim`
  (bind (_startantennatransform_location _startantennatransform_rotation _startantennatransform_scale) (`KismetMathLibrary.BreakTransform` (`self.StartAntennaTransform`)))
  (set `self.StartAntennaTransform` (`SceneComponent.GetRelativeTransform` (`self.Antenna`)))
  (bind (_direction _newtrack_0) (`Timeline|AntennaTimeline`)
    (:`Update`
      (`SceneComponent.K2_SetRelativeTransform` (`self.Antenna`) (`KismetMathLibrary.MakeTransform` _startantennatransform_location (`KismetMathLibrary.RLerp` _startantennatransform_rotation (`self.AntennaRotation`) _newtrack_0) _startantennatransform_scale) false false))
    (:`Finished`
      (`self.BeamOn`))))

(fn `UserConstructionScript`)