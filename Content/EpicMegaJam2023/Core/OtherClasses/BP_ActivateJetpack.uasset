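; BP_ActivateJetpack is a trigger volume that forces the jetpack on for a set duration when an actor with AC_JetPack overlaps its box.
; On overlap it stores the component, turns off its stamina requirement and starts a looping timer, apparently bound to ActivateJetpack, to drive the action.
; A one-shot timer then clears the loop and deactivates the jetpack, without restoring the stamina requirement here.
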(event `self.Box.OnComponentBeginOverlap`
  (params (OverlappedComponent :type "PrimitiveComponent Object Reference") (OtherActor :type "Actor Object Reference") (OtherComp :type "PrimitiveComponent Object Reference") (OtherBodyIndex :type Integer) (bFromSweep :type Boolean) (SweepResult :type "HitResult Structure (by ref)"))
  (bind _returnvalue (`self.GetComponentByClass` OtherActor "/Game/EpicMegaJam2023/Core/Components/Items/AC_JetPack.AC_JetPack_C"))
  (`/Engine/EditorBlueprintResources/StandardMacros.IsValid` _returnvalue
    (:`Is Valid`
      (bind _output_get (set `self.JetPackComponent` _returnvalue))
      (set `/Game/EpicMegaJam2023/Core/Components/AC_BaseItemComponent.bNeedStamina` false _output_get)
      (bind _returnvalue_2 (`KismetSystemLibrary.K2_SetTimerDelegate` (`|CreateDelegate` :!event `ActivateJetpack`) (`self.Time`) true))
      (set `self.TimerStopJetPack` _returnvalue_2)
      (`KismetSystemLibrary.K2_SetTimerDelegate` (delegate `CanActivate`) (`self.TimerDuration`)))))

(event `CanActivate`
  (`KismetSystemLibrary.K2_ClearAndInvalidateTimerHandle` (`self.TimerStopJetPack`))
  (`/Game/EpicMegaJam2023/Core/Components/AC_BaseItemComponent.DeactivateAction` (`self.JetPackComponent`)))

(fn `ActivateJetpack`
  (`/Game/EpicMegaJam2023/Core/Components/AC_BaseItemComponent.ActivateAction` (`self.JetPackComponent`)))

(fn `UserConstructionScript`)