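; Actor that endlessly rotates two static mesh components in opposite yaw directions from BeginPlay.
; A single Timeline track drives both relative yaws, with its sign swapped between meshes and flipped again when the Timeline plays backward.
; The Timeline's Finished output feeds back into a FlipFlop, alternating PlayFromStart and ReverseFromEnd in a continuous loop.
; An unconnected node that zeroes CustomTimeDilation never runs.
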(event `self.ReceiveBeginPlay`
  (`self.CustomEvent`))

(event `CustomEvent`
  (`/Engine/EditorBlueprintResources/StandardMacros.FlipFlop` :!label _label
    (:`A`
      (bind (_direction _newtrack_0) (`Timeline|Timeline` :!via `PlayFromStart` :!label _label_2)
        (:`Update`
          (`SceneComponent.K2_SetRelativeRotation` (`self.StaticMesh1`) (`KismetMathLibrary.MakeRotator` 0.0 0.0 (select `ETimelineDirection` _direction :`Forward` (* _newtrack_0 1.0) :`Backward` (* -1.0 _newtrack_0))) false false)
          (`SceneComponent.K2_SetRelativeRotation` (`self.StaticMesh`) (`KismetMathLibrary.MakeRotator` 0.0 0.0 (select `ETimelineDirection` _direction :`Forward` (* _newtrack_0 -1.0) :`Backward` (* _newtrack_0 1.0))) false false))
        (:`Finished`
          (goto _label))))
    (:`B`
      (goto _label_2 :!via `ReverseFromEnd`))))

(fn `UserConstructionScript`)