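; BP_TestActor is a utility test actor that batch-fixes collision on wall meshes so they get the NoClimbable profile.
; Its SetWallProfileCollision event scans every StaticMeshActor, sets that collision profile on those using the Wall_02 mesh, and prints each one's name and index.
; Nothing in the file calls the event, and a roll-angle filter for 180-degree rotated walls is left unconnected.
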(event `SetWallProfileCollision`
  (bind _outactors (`GameplayStatics.GetAllActorsOfClass` "/Script/Engine.StaticMeshActor"))
  (for (_array_element _array_index) _outactors
    (if (== (`StaticMeshComponent.StaticMesh` (`StaticMeshActor.StaticMeshComponent` _array_element)) "/Game/EpicMegaJam2023/Art/Furniture/Floor_And_Walls/Wall_02.Wall_02")
      (`KismetSystemLibrary.PrintString` (`KismetSystemLibrary.GetDisplayName` _array_element))
      (`KismetSystemLibrary.PrintString` (`KismetStringLibrary.Conv_IntToString` _array_index))
      (`PrimitiveComponent.SetCollisionProfileName` (`StaticMeshActor.StaticMeshComponent` _array_element) "NoClimbable" true))))

(fn `UserConstructionScript`)