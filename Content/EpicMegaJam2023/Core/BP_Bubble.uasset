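; BP_Bubble is a bubble actor that bobs up and down continuously at a randomized size.
; BeginPlay gives the static mesh a random uniform scale, then a FlipFlop alternates a timeline between forward and reverse, re-triggering whenever it finishes.
; Each update nudges the mesh along relative Z, with sign set by playback direction and step size by the curve.
; ToggleState destroys the actor when passed true.
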(event `self.ReceiveBeginPlay`
  (`SceneComponent.SetRelativeScale3D` (`self.StaticMesh`) (`KismetMathLibrary.Conv_DoubleToVector` (`KismetMathLibrary.RandomFloatInRange` 0.1 0.5)))
  (`/Engine/EditorBlueprintResources/StandardMacros.FlipFlop` :!label _label
    (:`A`
      (bind (_direction _newtrack_0) (`Timeline|Timeline` :!via `PlayFromStart` :!label _label_2)
        (:`Update`
          (`SceneComponent.K2_AddRelativeLocation` (`self.StaticMesh`) (`KismetMathLibrary.VLerp` (0.0 0.0 0.0) (select `ETimelineDirection` _direction :`Forward` (0.0 0.0 1.0) :`Backward` (0.0 0.0 -1.0) :!type "Vector Structure") _newtrack_0) false false))
        (:`Finished`
          (goto _label))))
    (:`B`
      (goto _label_2 :!via `ReverseFromEnd`))))

(event `/Game/EpicMegaJam2023/Core/Interfaces/BPI_LaserInterface.ToggleState`
  (params (`On/Off` :type Boolean))
  (if `On/Off`
    (`self.K2_DestroyActor`)))

(fn `UserConstructionScript`)