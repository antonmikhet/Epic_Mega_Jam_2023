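; Actor component for the main character that tracks the last checkpoint and respawns the player there on a kill event.
; It starts from FirstCheckPoint, printing a message if that is unset, and exposes a setter for later checkpoints.
; EventKill changes the input state, fades the camera out, then teleports the owner to the checkpoint's spawn transform.
; Timers and self-bound event dispatchers chain the hold, fade back in and input reset.
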(event `self.ReceiveBeginPlay`
  (bind _output (`|ConvertAsset` (`self.FirstCheckPoint`)))
  (`/Engine/EditorBlueprintResources/StandardMacros.IsValid` _output
    (:`Is Valid`
      (`self.SetCheckPointActor` _output))
    (:`Is Not Valid`
      (`KismetSystemLibrary.PrintString` "First Checkpoint nullptr" true true (struct :`R` 1.0 :`B` 0.017682 :`A` 1.0))))
  (bind _asch_main_character (cast `/Game/EpicMegaJam2023/Core/Character/MainCharacter/CH_MainCharacter` (`self.GetOwner`)))
  (set `self.Owner` _asch_main_character))

(event `EventKill`
  (`/Game/EpicMegaJam2023/Core/Character/MainCharacter/CH_MainCharacter.SetInputStates` (`self.Owner`) "NewEnumerator2")
  (`self.EventFadeIn`))

(event `OnFadeOut_Event`
  (`PlayerCameraManager.StartCameraFade` :`self` (`self.GetPlayerCameraManager`) :`FromAlpha` 1.0 :`Duration` 0.5)
  (`/Game/EpicMegaJam2023/Core/Character/MainCharacter/CH_MainCharacter.SetInputStates` (`self.Owner`) "NewEnumerator0"))

(event `OnFadeIn_Event`
  (`PlayerCameraManager.StartCameraFade` :`self` (`self.GetPlayerCameraManager`) :`FromAlpha` 1.0 :`ToAlpha` 1.0 :`Duration` 1.0)
  (`KismetSystemLibrary.K2_SetTimerDelegate` (delegate `CallFadeOut`) 0.9))

(event `CallFadeOut`
  (`self.OnFadeOut`))

(event `EventFadeIn`
  (`|ExecutionSequence`
    (:`then_0`
      (add `self.OnFadeIn` (delegate `OnFadeIn_Event`))
      (add `self.OnFadeOut` (delegate `OnFadeOut_Event`)))
    (:`then_1`
      (`PlayerCameraManager.StartCameraFade` :`self` (`self.GetPlayerCameraManager`) :`ToAlpha` 1.0 :`Duration` 0.6)
      (`KismetSystemLibrary.K2_SetTimerDelegate` (delegate `CallFadeIn`) 0.5))))

(event `CallFadeIn`
  (bind (_returnvalue_location _returnvalue_rotation) (`KismetMathLibrary.BreakTransform` (`self.GetSpawnPosition`)))
  (`Actor.K2_SetActorLocationAndRotation` (`self.GetOwner`) _returnvalue_location _returnvalue_rotation false false)
  (`self.OnFadeIn`))

(fn `GetCheckPointActor`
  (returns (LastCheckPointActor :type "/Game/EpicMegaJam2023/Core/OtherClasses/CheckPoint/BP_CheckPoint Object Reference"))
  (return (`self.LastCheckPointActor`)))

(fn `GetPlayerCameraManager`
  (returns (PlayerCameraManager :type "PlayerCameraManager Object Reference"))
  (return (`PlayerController.PlayerCameraManager` (`Pawn.GetLocalViewingPlayerController` (cast `Character` (`self.GetOwner`) :!pure true)))))

(fn `GetSpawnPosition`
  (returns (ReturnValue :type "Transform Structure"))
  (return (`/Game/EpicMegaJam2023/Core/OtherClasses/CheckPoint/BP_CheckPoint.GetSpawnPosition` (`self.GetCheckPointActor`))))

(fn `SetCheckPointActor`
  (params (LastCheckPointActor :type "/Game/EpicMegaJam2023/Core/OtherClasses/CheckPoint/BP_CheckPoint Object Reference"))
  (set `self.LastCheckPointActor` LastCheckPointActor))