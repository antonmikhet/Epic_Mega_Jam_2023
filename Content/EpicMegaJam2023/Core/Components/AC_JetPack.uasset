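; AC_JetPack is an action component that gives the main character an upward jet pack boost.
; On activation it casts its owner to CH_MainCharacter, stores the reference and applies a single mass-dependent vertical impulse through the character movement component.
; Deactivation only calls the parent implementation, and the component runs no per-frame thrust or fuel logic.
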(fn `ActivateAction`
  (`parent.ActivateAction`)
  (bind _asch_main_character (cast `/Game/EpicMegaJam2023/Core/Character/MainCharacter/CH_MainCharacter` (`self.GetOwner`)))
  (bind _output_get (set `self.CHMainCharacter_0` _asch_main_character))
  (`CharacterMovementComponent.AddImpulse` (`Character.CharacterMovement` _output_get) (0.0 0.0 4000.0) false))

(fn `DeactivateAction`
  (`parent.DeactivateAction`))