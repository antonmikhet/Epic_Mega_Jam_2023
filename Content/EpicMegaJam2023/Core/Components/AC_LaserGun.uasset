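; Action component for the main character's laser gun, firing a beam that bounces off mirrors and switches on laser sensors.
; While active, it sets the aim state and runs a looping timer to update the laser.
; The beam runs from a mesh socket toward the camera's aim point.
; CastLight repeatedly line-traces, identifying mirrors and sensors by hit-face material, and rebuilds BP_LaserBeam actors per segment, resetting the sensor on each rebuild.
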(event `self.ReceiveTick`
  (params (DeltaSeconds :type "Float (single-precision)"))
  (`parent.ReceiveTick` DeltaSeconds))

(fn `ActivateAction`
  (`parent.ActivateAction`)
  (bind _returnvalue (`KismetSystemLibrary.K2_SetTimerDelegate` (`|CreateDelegate` :!event `LaserEvent`) (`self.TimeToUpdateLaser`) true))
  (set `self.LaserTimer` _returnvalue)
  (set `/Game/EpicMegaJam2023/Core/Character/MainCharacter/CH_MainCharacter.AimState` true (`self.CHMainCharacter`))
  (return))

(fn `CalculateLaserBeamParams`
  (returns (Origin :type "Vector Structure") (CastDirection :type "Vector Structure"))
  (bind _followcamera (`/Game/EpicMegaJam2023/Core/Character/MainCharacter/ThirdPerson/Blueprints/BP_ThirdPersonCharacter.FollowCamera` (`self.CHMainCharacter`)))
  (bind _returnvalue (`SceneComponent.GetSocketLocation` (`Character.Mesh` (`self.CHMainCharacter`)) (`KismetStringLibrary.Conv_StringToName` (`self.SocketName`))))
  (bind _returnvalue_2 (`SceneComponent.K2_GetComponentLocation` _followcamera))
  (bind _returnvalue_3 (+ _returnvalue_2 (* (`SceneComponent.GetForwardVector` _followcamera) 100000000.0)))
  (bind (_outhit _returnvalue_4) (`KismetSystemLibrary.LineTraceSingle` _returnvalue_2 _returnvalue_3 "TraceTypeQuery1"))
  (return _returnvalue (`KismetMathLibrary.GetDirectionUnitVector` _returnvalue (select `bool` _returnvalue_4 :`false` _returnvalue_3 :`true` (`.ImpactPoint` (`GameplayStatics.BreakHitResult` _outhit))))))

(fn `CastLight`
  (params (CastOrigin :type "Vector Structure") (CastDirection :type "Vector Structure") (CastDistance :type "Float (double-precision)" :default 1000000000.0))
  (locals (Continue :type Boolean :default true) (LocBeamEnd :type "Vector Structure") (LocBeamStart :type "Vector Structure"))
  (bind _castorigin (`local.CastOrigin`))
  (bind _castdirection (`local.CastDirection`))
  (bind _returnvalue (+ _castorigin (* (`local.CastDirection`) (`local.CastDistance`))))
  (`self.DestroyBeams`)
  (while (`local.Continue`)
    (`|ExecutionSequence`
      (:`then_0`
        (bind (_outhit _returnvalue_2) (`KismetSystemLibrary.LineTraceSingle` _castorigin _returnvalue "TraceTypeQuery3" true))
        (set `local.LocBeamStart` (`local.CastOrigin`))
        (set `local.LocBeamEnd` _returnvalue)
        (if _returnvalue_2
          (bind (_bblockinghit _binitialoverlap _time _distance _location _impactpoint _normal _impactnormal _physmat _hitactor _hitcomponent _hitbonename _bonename _hititem _elementindex _faceindex) (`GameplayStatics.BreakHitResult` _outhit))
          (set `local.LocBeamEnd` _impactpoint)
          (bind (_sectionindex _returnvalue_3) (`PrimitiveComponent.GetMaterialFromCollisionFaceIndex` _hitcomponent _faceindex))
          (if (== _returnvalue_3 "/Game/EpicMegaJam2023/MaterialLibrary/MasterMaterials/M_MirrorMaterial.M_MirrorMaterial")
            (`KismetMathLibrary.Vector_Set` (`local.CastOrigin`) (.x _impactpoint) (.y _impactpoint) (.z _impactpoint))
            (`KismetMathLibrary.Vector_Set` _castdirection (.x (`KismetMathLibrary.MirrorVectorByNormal` _castdirection _impactnormal)) (.y (`KismetMathLibrary.MirrorVectorByNormal` _castdirection _impactnormal)) (.z (`KismetMathLibrary.MirrorVectorByNormal` _castdirection _impactnormal)))
            (set `local.Continue` true)
            (else
              (`/Engine/EditorBlueprintResources/StandardMacros.IsValid` _hitactor :!label _label
                (:`Is Valid`
                  (if (== _returnvalue_3 "/Game/EpicMegaJam2023/MaterialLibrary/MasterMaterials/M_LaserSensor.M_LaserSensor")
                    (bind _output_get (set `self.ActivatedSensor` _hitactor))
                    (message `/Game/EpicMegaJam2023/Core/Interfaces/BPI_LaserInterface.ToggleState` _output_get true)
                    (set `local.Continue` false)
                    (else
                      (set `local.Continue` false)))))))
          (else
            (set `local.Continue` false)
            (goto _label))))
      (:`then_1`
        (bind _returnvalue_4 (`|SpawnActorFromClass` "/Game/EpicMegaJam2023/Core/OtherClasses/Laser/BP_LaserBeam.BP_LaserBeam_C" (`KismetMathLibrary.MakeTransform` (0.0 0.0 0.0)) "AlwaysSpawn" "MultiplyWithRoot" null null))
        (`Actor.SetActorHiddenInGame` _returnvalue_4 true)
        (`/Game/EpicMegaJam2023/Core/OtherClasses/Laser/BP_LaserBeam.SetEnds` _returnvalue_4 (`local.LocBeamStart`) (`local.LocBeamEnd`))
        (`Actor.SetActorHiddenInGame` _returnvalue_4 false)
        (`KismetArrayLibrary.Array_Add` (`self.Beams`) _returnvalue_4)))))

(fn `DeactivateAction`
  (bind _chmaincharacter (`self.CHMainCharacter`))
  (`parent.DeactivateAction`)
  (`KismetSystemLibrary.K2_ClearAndInvalidateTimerHandle` (`self.LaserTimer`))
  (`self.DestroyBeams`)
  (if (not (`/Game/EpicMegaJam2023/Core/Character/MainCharacter/CH_MainCharacter.AimKeyIsDown` _chmaincharacter))
    (set `/Game/EpicMegaJam2023/Core/Character/MainCharacter/CH_MainCharacter.AimState` false _chmaincharacter)))

(fn `DestroyBeams`
  (for _array_element (`self.Beams`)
    (`Actor.K2_DestroyActor` _array_element))
  (`KismetArrayLibrary.Array_Clear` (`self.Beams`))
  (message `/Game/EpicMegaJam2023/Core/Interfaces/BPI_LaserInterface.ToggleState` (`self.ActivatedSensor`) false))

(fn `LaserEvent`
  (bind (_origin _castdirection) (`self.CalculateLaserBeamParams`))
  (`self.CastLight` _origin _castdirection (`self.Cast Distance`)))