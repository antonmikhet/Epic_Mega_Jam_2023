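; AC_TimeDilation is an item component whose action slows a BP_EpicMegaJam2023Actor in time while active.
; It extends the parent's activate and deactivate actions, then finds that actor by class and sets its CustomTimeDilation.
; Activation sets normal speed and deactivation restores a heavily accelerated rate, so the slowdown is relative.
; Global time dilation nodes remain in both graphs but never run.
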(fn `ActivateAction`
  (`parent.ActivateAction`)
  (bind _returnvalue (`GameplayStatics.GetActorOfClass` "/Game/EpicMegaJam2023/Core/OtherClasses/BP_EpicMegaJam2023Actor.BP_EpicMegaJam2023Actor_C"))
  (set `Actor.CustomTimeDilation` 1.0 _returnvalue))

(fn `DeactivateAction`
  (`parent.DeactivateAction`)
  (bind _returnvalue (`GameplayStatics.GetActorOfClass` "/Game/EpicMegaJam2023/Core/OtherClasses/BP_EpicMegaJam2023Actor.BP_EpicMegaJam2023Actor_C"))
  (set `Actor.CustomTimeDilation` 20.0 _returnvalue))