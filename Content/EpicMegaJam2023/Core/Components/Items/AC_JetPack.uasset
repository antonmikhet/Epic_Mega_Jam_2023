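; Jetpack item component that pushes the main character with a movement force when its action activates.
; Activation also plays a camera shake, starts the character's Niagara effect and changes the aim offset; deactivation stops the effect and restores the offset.
; Equipping attaches a cylinder mesh to the StaminaSocket with a dynamic circle material, which Tick updates as a stamina gauge.
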(event `self.ReceiveTick`
  (params (DeltaSeconds :type "Float (single-precision)"))
  (bind _staminamaterial (`self.StaminaMaterial`))
  (`parent.ReceiveTick` DeltaSeconds)
  (`/Engine/EditorBlueprintResources/StandardMacros.IsValid` _staminamaterial
    (:`Is Valid`
      (`MaterialInstanceDynamic.SetScalarParameterValue` _staminamaterial "Percent" (`KismetMathLibrary.MapRangeClamped` (`self.StaminaCurrent`) 0.0 100.0 0.0 1.0)))))

(fn `ActivateAction`
  (`parent.ActivateAction`)
  (`GameplayStatics.PlayWorldCameraShake` "/Game/EpicMegaJam2023/Core/Engine/CameraShake/CS_JetPack.CS_JetPack_C" (`Actor.K2_GetActorLocation` (`self.GetOwner`)) 500.0 500.0)
  (`/Game/EpicMegaJam2023/Core/Character/MainCharacter/CH_MainCharacter.SetAimOffset` (`self.CHMainCharacter`) 80.0)
  (`/Game/EpicMegaJam2023/Core/Character/MainCharacter/CH_MainCharacter.ActivateNiagaraSystem` (`self.CHMainCharacter`))
  (`CharacterMovementComponent.AddForce` (`Character.CharacterMovement` (`self.CHMainCharacter`)) (* (`self.Force`) 1000.0)))

(fn `DeactivateAction`
  (`parent.DeactivateAction`)
  (`/Game/EpicMegaJam2023/Core/Character/MainCharacter/CH_MainCharacter.DeactivateNiagaraSystem` (`self.CHMainCharacter`))
  (`/Game/EpicMegaJam2023/Core/Character/MainCharacter/CH_MainCharacter.SetDefaultAimOffset` (`self.CHMainCharacter`)))

(fn `PutOnItem`
  (bind _chmaincharacter (`self.CHMainCharacter`))
  (`parent.PutOnItem`)
  (bind _returnvalue (`|AddComponentByClass` _chmaincharacter "/Script/Engine.StaticMeshComponent" false (`KismetMathLibrary.MakeTransform` (0.0 0.0 0.0))))
  (`StaticMeshComponent.SetStaticMesh` _returnvalue "/Engine/BasicShapes/Cylinder.Cylinder")
  (`SceneComponent.K2_AttachToComponent` _returnvalue (`Actor.GetComponentByClass` _chmaincharacter "/Script/Engine.SkeletalMeshComponent") "StaminaSocket" "SnapToTarget" "SnapToTarget" "SnapToTarget" true)
  (bind _returnvalue_2 (`PrimitiveComponent.CreateDynamicMaterialInstance` _returnvalue 0 "/Game/EpicMegaJam2023/MaterialLibrary/M_CircleMaterial_Inst.M_CircleMaterial_Inst" "None"))
  (set `self.StaminaMaterial` _returnvalue_2))