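; Base item component with a stamina-limited action and an empty PutOnItem function, apparently meant for extension by specific items.
; PreActivationAction calls ActivateAction, which starts a looping one-second timer draining stamina if any remains, and returns false either way.
; DeactivateAction clears that timer and starts a looping regeneration timer, but StaminaIncrement only pauses the drain timer, leaving its refill logic unreachable.
; Debug prints trace activation and stamina.
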(fn `ActivateAction`
  (returns (NewParam :type Boolean))
  (if (> (`self.StaminaCurrent`) 0.0)
    (if (not (`KismetSystemLibrary.K2_IsTimerActiveHandle` (`self.StaminaActivationTimer`)))
      (bind _returnvalue (`KismetSystemLibrary.K2_SetTimer` null "StaminaDecrement" 1.0 true))
      (set `self.StaminaActivationTimer` _returnvalue))
    (`KismetSystemLibrary.PrintString` (`KismetStringLibrary.Concat_StrStr` "ActivateAction " (`KismetSystemLibrary.GetDisplayName` self)) true true (struct :`G` 0.66 :`B` 1.0 :`A` 1.0) 2.0 "r")
    (`KismetSystemLibrary.PrintString` (`KismetStringLibrary.Conv_DoubleToString` (`self.StaminaCurrent`)) true true (struct :`G` 0.66 :`B` 1.0 :`A` 1.0) 1000.0 "e")
    (return false)
    (else
      (return false))))

(fn `DeactivateAction`
  (bind _staminaactivationtimer (`self.StaminaActivationTimer`))
  (`KismetSystemLibrary.K2_PauseTimerHandle` _staminaactivationtimer)
  (`KismetSystemLibrary.K2_ClearAndInvalidateTimerHandle` _staminaactivationtimer)
  (bind _returnvalue (`KismetSystemLibrary.K2_SetTimer` null "StaminaIncrement" 1.0 true))
  (set `self.StaminaDeactivateTimer` _returnvalue)
  (`KismetSystemLibrary.PrintString` (`KismetStringLibrary.Concat_StrStr` "DeactivateAction " (`KismetSystemLibrary.GetDisplayName` self))))

(fn `PreActivationAction`
  (`self.ActivateAction`))

(fn `PutOnItem`)

(fn `StaminaDecrement`
  (bind _output_get (set `self.StaminaCurrent` (- (`self.StaminaCurrent`) (`self.StaminaDe`))))
  (`KismetSystemLibrary.PrintString` (`KismetStringLibrary.Conv_DoubleToString` _output_get) true true (struct :`G` 0.66 :`B` 1.0 :`A` 1.0) 100.0 "g"))

(fn `StaminaIncrement`
  (if true
    (`KismetSystemLibrary.K2_PauseTimerHandle` (`self.StaminaActivationTimer`))))