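; AC_HealthComponent is an actor component that tracks health for its owner.
; On BeginPlay it fills current health to max and binds its own handler to the OnHealthEmpty dispatcher.
; DecreaseHealth subtracts damage while health is above zero, clamps at zero and fires OnHealthEmpty when depleted.
; The built-in empty handler only prints a debug message, and getters expose current and max health.
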(event `self.ReceiveBeginPlay`
  (`self.SetCurrentHealth` (`self.GetMaxHealth`))
  (add `self.OnHealthEmpty` (`|CreateDelegate` :!event `EventOnHealthEmpty`)))

(fn `DecreaseHealth`
  (params (Damage :type "Float (double-precision)"))
  (if (> (`self.CurrentHealth`) 0.0)
    (bind _output_get (set `self.CurrentHealth` (- (`self.CurrentHealth`) Damage)))
    (if (<= _output_get 0.0)
      (set `self.CurrentHealth` 0.0)
      (`self.OnHealthEmpty`))))

(fn `EventOnHealthEmpty`
  (`KismetSystemLibrary.PrintString` "HealthWasEmpty"))

(fn `GetCurrentHealth`
  (returns (CurrentHealth :type "Float (double-precision)"))
  (return (`self.CurrentHealth`)))

(fn `GetMaxHealth`
  (returns (MaxHealth :type "Float (double-precision)"))
  (return (`self.MaxHealth`)))

(fn `SetCurrentHealth`
  (params (CurrentHealth :type "Float (double-precision)"))
  (set `self.CurrentHealth` CurrentHealth))