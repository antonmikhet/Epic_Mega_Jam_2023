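; Actor component for the main character that applies a toxic debuff, slowing movement, jump and mouse sensitivity and changing input state.
; Damage adds to a toxic count shown on a toxic HUD widget, then delayed timers after last contact end the effect using settings cached at BeginPlay.
; Looping timers can raise or drain the count over time.
; Reaching maximum fires a kill event handled by the checkpoint system component.
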(event `self.ReceiveBeginPlay`
  (bind _asch_main_character (cast `/Game/EpicMegaJam2023/Core/Character/MainCharacter/CH_MainCharacter` (`self.GetOwner`)))
  (bind _output_get (set `self.As CH Main Character` _asch_main_character))
  (bind _returnvalue (`|GenericCreateObject` _output_get "/Game/EpicMegaJam2023/Core/UI/ToxicHUD/WB_ToxicHUD.WB_ToxicHUD_C"))
  (bind _output_get_2 (set `self.ToxicHud` _returnvalue))
  (`UserWidget.AddToViewport` _output_get_2 0)
  (add `self.OnKillEvent` (`|CreateDelegate` :!event `EventOnKillEvent`))
  (`self.SetDefaultPrimaryCharacterSettings`))

(fn `Damage`
  (params (Damage :type "Float (double-precision)"))
  (`self.StartToxicEffect`)
  (if (> (+ (`local.Damage`) (`self.GetCurrentToxicCount`)) (`self.GetMaxToxicCount`))
    (`self.SetCurrentToxicCount` (`self.GetMaxToxicCount`))
    (`self.OnKillEvent`)
    (`self.SetToxicHUDEffect`)
    (else
      (`self.SetCurrentToxicCount` (+ (`local.Damage`) (`self.GetCurrentToxicCount`)))
      (`self.SetToxicHUDEffect`)
      (`self.EndToxicEffect` true))))

(fn `DecrementToxicEffect`
  (if (> (`self.GetCurrentToxicCount`) 0.0)
    (`self.SetCurrentToxicCount` (- (`self.GetCurrentToxicCount`) (`self.DecrementTick`)))
    (`self.SetToxicHUDEffect`)
    (else
      (`self.SetCurrentToxicCount` 0.0)
      (`self.SetToxicHUDEffect`)
      (`self.StopTimerDecrementToxicEffect`))))

(fn `EndToxicEffect`
  (params (bWithTimer :type Boolean :default true))
  (if bWithTimer
    (`KismetSystemLibrary.K2_SetTimerDelegate` (`|CreateDelegate` :!event `SetPrimaryCharacterSettings`) (`self.TimeAfterLastContact`))
    (else
      (`self.SetPrimaryCharacterSettings`)))
  (if (`KismetSystemLibrary.K2_IsValidTimerHandle` (`self.TimerAfterLastDamage`))
    (`KismetSystemLibrary.K2_ClearAndInvalidateTimerHandle` (`self.TimerAfterLastDamage`)))
  (bind _returnvalue (`KismetSystemLibrary.K2_SetTimerDelegate` (`|CreateDelegate` :!event `StartTimertDecrementToxicEffect`) (`self.TimeAfterLastContact`)))
  (set `self.TimerAfterLastDamage` _returnvalue))

(fn `EventOnKillEvent`
  (bind _returnvalue (`Actor.GetComponentByClass` (`self.As CH Main Character`) "/Game/EpicMegaJam2023/Core/Components/AC_CheckPointSystem.AC_CheckPointSystem_C"))
  (`/Engine/EditorBlueprintResources/StandardMacros.IsValid` _returnvalue
    (:`Is Valid`
      (`/Game/EpicMegaJam2023/Core/Components/AC_CheckPointSystem.EventKill` _returnvalue))))

(fn `GetCurrentToxicCount`
  (returns (CurrentToxicCount :type "Float (double-precision)"))
  (return (`self.CurrentToxicCount`)))

(fn `GetMaxToxicCount`
  (returns (MaxToxicCount :type "Float (double-precision)"))
  (return (`self.MaxToxicCount`)))

(fn `IncrementToxicEffect`
  (if (< (`self.GetCurrentToxicCount`) (`self.GetMaxToxicCount`))
    (`self.SetCurrentToxicCount` (+ (`self.GetCurrentToxicCount`) (`self.IncrementTick`)))
    (`self.SetToxicHUDEffect`)
    (else
      (`self.SetCurrentToxicCount` (`self.GetMaxToxicCount`))
      (`self.SetToxicHUDEffect`)
      (`self.StopTimerIncrementToxicEffect`)
      (`self.OnKillEvent`))))

(fn `SetCurrentToxicCount`
  (params (CurrentToxicCount :type "Float (double-precision)"))
  (set `self.CurrentToxicCount` CurrentToxicCount))

(fn `SetDefaultPrimaryCharacterSettings`
  (bind _as_ch_main_character (`self.As CH Main Character`))
  (bind _charactermovement (`Character.CharacterMovement` _as_ch_main_character))
  (set `self.PrimaryMaxWalkSpeed` (`CharacterMovementComponent.MaxWalkSpeed` _charactermovement))
  (set `self.PrimaryJumpZVelocity` (`CharacterMovementComponent.JumpZVelocity` _charactermovement))
  (set `self.PrimaryMouseSensitivity` (`/Game/EpicMegaJam2023/Core/Character/MainCharacter/CH_MainCharacter.MouseSensitivity` _as_ch_main_character)))

(fn `SetPrimaryCharacterSettings`
  (bind _charactermovement (`Character.CharacterMovement` (`self.As CH Main Character`)))
  (set `CharacterMovementComponent.MaxWalkSpeed` (`self.PrimaryMaxWalkSpeed`) _charactermovement)
  (set `CharacterMovementComponent.JumpZVelocity` (`self.PrimaryJumpZVelocity`) _charactermovement)
  (set `/Game/EpicMegaJam2023/Core/Character/MainCharacter/CH_MainCharacter.MouseSensitivity` (`self.PrimaryMouseSensitivity`) (`self.As CH Main Character`))
  (`/Game/EpicMegaJam2023/Core/Character/MainCharacter/CH_MainCharacter.SetInputStates` (`self.As CH Main Character`) "NewEnumerator0"))

(fn `SetToxicHUDEffect`
  (`/Game/EpicMegaJam2023/Core/UI/ToxicHUD/WB_ToxicHUD.SetToxicAlpha` (`self.ToxicHud`) (`self.GetCurrentToxicCount`) (`self.GetMaxToxicCount`)))

(fn `StartTimertDecrementToxicEffect`
  (bind _returnvalue (`KismetSystemLibrary.K2_SetTimerDelegate` (`|CreateDelegate` :!event `DecrementToxicEffect`) 0.1 true))
  (set `self.DecrementToxicEffectTimer` _returnvalue))

(fn `StartTimertIncrementToxicEffect`
  (bind _returnvalue (`KismetSystemLibrary.K2_SetTimerDelegate` (`|CreateDelegate` :!event `IncrementToxicEffect`) 0.1 true))
  (set `self.IncrementToxicEffectTimer` _returnvalue))

(fn `StartToxicEffect`
  (bind _charactermovement (`Character.CharacterMovement` (`self.As CH Main Character`)))
  (set `CharacterMovementComponent.MaxWalkSpeed` (`self.ToxicMaxWalkSpeed`) _charactermovement)
  (set `CharacterMovementComponent.JumpZVelocity` (`self.ToxicJumpZVelocity`) _charactermovement)
  (set `/Game/EpicMegaJam2023/Core/Character/MainCharacter/CH_MainCharacter.MouseSensitivity` (`self.ToxicMouseSensitivity`) (`self.As CH Main Character`))
  (`/Game/EpicMegaJam2023/Core/Character/MainCharacter/CH_MainCharacter.SetInputStates` (`self.As CH Main Character`) "NewEnumerator3"))

(fn `StopTimerDecrementToxicEffect`
  (`KismetSystemLibrary.K2_ClearAndInvalidateTimerHandle` (`self.DecrementToxicEffectTimer`)))

(fn `StopTimerIncrementToxicEffect`
  (`KismetSystemLibrary.K2_ClearAndInvalidateTimerHandle` (`self.IncrementToxicEffectTimer`)))