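; BP_ToxicAreaActor is an area actor that applies a toxic debuff to the main character while inside its Box volume.
; On begin overlap it casts to CH_MainCharacter, adds an AC_ToxicEffect component and caches both references.
; On end overlap by that character, it calls EndEffect on the component found by the cached effect's class, which may not be the cached instance.
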(event `self.Box.OnComponentBeginOverlap`
  (params (OverlappedComponent :type "PrimitiveComponent Object Reference") (OtherActor :type "Actor Object Reference") (OtherComp :type "PrimitiveComponent Object Reference") (OtherBodyIndex :type Integer) (bFromSweep :type Boolean) (SweepResult :type "HitResult Structure (by ref)"))
  (bind _asch_main_character (cast `/Game/EpicMegaJam2023/Core/Character/MainCharacter/CH_MainCharacter` OtherActor))
  (bind _output_get (set `self.As CH Main Character` _asch_main_character))
  (bind _returnvalue (`|AddComponentByClass` _output_get "/Game/EpicMegaJam2023/Core/Components/DebufEffects/EffectsComponents/AC_ToxicEffect.AC_ToxicEffect_C"))
  (set `self.EffectComponent` _returnvalue))

(event `self.Box.OnComponentEndOverlap`
  (params (OverlappedComponent :type "PrimitiveComponent Object Reference") (OtherActor :type "Actor Object Reference") (OtherComp :type "PrimitiveComponent Object Reference") (OtherBodyIndex :type Integer))
  (bind _effectcomponent (`self.EffectComponent`))
  (bind _as_ch_main_character (`self.As CH Main Character`))
  (if (== OtherActor _as_ch_main_character)
    (`/Engine/EditorBlueprintResources/StandardMacros.IsValid` _effectcomponent
      (:`Is Valid`
        (`/Game/EpicMegaJam2023/Core/Components/DebufEffects/EffectsComponents/AC_ToxicEffect.EndEffect` (`self.GetComponentByClass` _as_ch_main_character (`GameplayStatics.GetObjectClass` _effectcomponent)))))))

(fn `UserConstructionScript`)