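; BP_Monument2_Elevator is a placeable elevator for the second monument that moves when its interaction event fires.
; A timeline, with play rate scaled by MoveTime, lerps the root's relative location from its BeginPlay position to ElevatorEndLocation.
; The interaction also sets the mesh material and calls every single-bubble and placeable bubble spawner in the level to spawn, the latter through its monument-exit spawn.
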(event `self.ReceiveBeginPlay`
  (`parent.ReceiveBeginPlay`)
  (`TimelineComponent.SetPlayRate` (`self.Timeline`) (/ 1.0 (`self.MoveTime`)))
  (set `self.ElevatorStartLocation` (`SceneComponent.RelativeLocation` (`self.Root`))))

(event `/Game/EpicMegaJam2023/Core/Interfaces/BPI_ItemInterface.EventInteraction`
  (params (Character :type "/Game/EpicMegaJam2023/Core/Character/MainCharacter/CH_MainCharacter Object Reference"))
  (`|ExecutionSequence`
    (:`then_0`
      (bind (_direction _newtrack_0) (`Timeline|Timeline`)
        (:`Update`
          (`SceneComponent.K2_SetRelativeLocation` (`self.Root`) (`KismetMathLibrary.VLerp` (`self.ElevatorStartLocation`) (`self.ElevatorEndLocation`) _newtrack_0) false false))))
    (:`then_1`
      (`PrimitiveComponent.SetMaterial` (`self.StaticMesh`) 0 null)
      (bind _outactors (`GameplayStatics.GetAllActorsOfClass` "/Game/EpicMegaJam2023/Core/Placeables/BP_SingleBubbleSpawner.BP_SingleBubbleSpawner_C"))
      (for _array_element _outactors
        (`/Game/EpicMegaJam2023/Core/Placeables/BP_SingleBubbleSpawner.SingleBubbleSpawn` _array_element)))
    (:`then_2`
      (bind _outactors_2 (`GameplayStatics.GetAllActorsOfClass` "/Game/EpicMegaJam2023/Placeables/BP_BubbleSpawner_Placeables.BP_BubbleSpawner_Placeables_C"))
      (for _array_element_2 _outactors_2
        (`/Game/EpicMegaJam2023/Core/OtherClasses/BP_BubbleSpawner.MonumentExitBubbleSpawn` _array_element_2)))))

(fn `UserConstructionScript`
  (`parent.UserConstructionScript`))