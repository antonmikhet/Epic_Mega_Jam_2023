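; A placeable laser-sensor double door that opens once its health is emptied.
; The parent's health-empty event calls StartAction, which removes a static mesh, plays cut and door sounds, and shatters the lock's Geometry Collection with a briefly spawned fracture field.
; A Timeline then slides both panels apart along relative X, with both targets computed from the left door's starting transform.
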(event `self.ReceiveBeginPlay`
  (`parent.ReceiveBeginPlay`)
  (set `self.DefaultTransformLeftDoor` (`SceneComponent.GetRelativeTransform` (`self.Scene_Left`)))
  (set `self.DefaultTransformRightDoor` (`SceneComponent.GetRelativeTransform` (`self.Scene_Right`)))
  (set `self.MeshLocation` (`SceneComponent.K2_GetComponentLocation` (`self.StaticMesh`))))

(event `self.StartAction`
  (bind _defaulttransformleftdoor (`self.DefaultTransformLeftDoor`))
  (bind _staticmesh (`self.StaticMesh`))
  (bind _defaulttransformleftdoor_2 (`self.DefaultTransformLeftDoor`))
  (`parent.StartAction`)
  (`/Engine/EditorBlueprintResources/StandardMacros.IsValid` _staticmesh
    (:`Is Valid`
      (`ActorComponent.K2_DestroyComponent` _staticmesh))
    (:`Is Not Valid`
      _))
  (`self.DestroyFractureMesh` (`self.Door_Lock_001_GeometryCollection`))
  (`GameplayStatics.PlaySoundAtLocation` "/Game/EpicMegaJam2023/Core/Audio/Metasounds/MS_Lazer_Cut.MS_Lazer_Cut" (`self.MeshLocation`) (struct) 1.0 1.0 0.0 null null null null)
  (`GameplayStatics.PlaySoundAtLocation` "/Game/EpicMegaJam2023/Core/Audio/Metasounds/MS_Doors.MS_Doors" (`SceneComponent.K2_GetComponentLocation` (`self.DefaultSceneRoot`)) (struct) 1.0 1.0 0.0 null null null null)
  (bind (_direction _newtrack_0) (`Timeline|Timeline`)
    (:`Update`
      (`SceneComponent.K2_SetRelativeTransform` (`self.Scene_Left`) (`KismetMathLibrary.TLerp` (`self.DefaultTransformLeftDoor`) (`KismetMathLibrary.MakeTransform` (`KismetMathLibrary.MakeVector` (+ (.x (.location _defaulttransformleftdoor)) -150.0) (.y (.location _defaulttransformleftdoor)) (.z (.location _defaulttransformleftdoor))) (.rotation _defaulttransformleftdoor) (.scale _defaulttransformleftdoor)) _newtrack_0) false false)
      (`SceneComponent.K2_SetRelativeTransform` (`self.Scene_Right`) (`KismetMathLibrary.TLerp` (`self.DefaultTransformRightDoor`) (`KismetMathLibrary.MakeTransform` (`KismetMathLibrary.MakeVector` (+ (.x (.location _defaulttransformleftdoor_2)) 150.0) (.y (.location _defaulttransformleftdoor_2)) (.z (.location _defaulttransformleftdoor_2))) (.rotation _defaulttransformleftdoor_2) (.scale _defaulttransformleftdoor_2)) _newtrack_0) false false))))

(fn `DestroyFractureMesh`
  (params (Component :type "PrimitiveComponent Object Reference"))
  (`PrimitiveComponent.SetSimulatePhysics` Component true)
  (bind _returnvalue (`|SpawnActorFromClass` "/Game/EpicMegaJam2023/Art/Fracture/FS_Fracture.FS_Fracture_C" (`KismetMathLibrary.MakeTransform` (- (`KismetSystemLibrary.GetComponentBounds` Component) (0.0 0.0 20.0)) (struct) (0.25 0.25 0.25)) "AlwaysSpawn" "MultiplyWithRoot" null null))
  (`/Engine/EditorResources/FieldNodes/FS_MasterField.CE_Trigger` _returnvalue)
  (`self.K2_DestroyActor` _returnvalue)
  (return))

(fn `OnHealthEmpty_Event`
  (`parent.OnHealthEmpty_Event`)
  (`self.StartAction`))

(fn `UserConstructionScript`
  (`parent.UserConstructionScript`))