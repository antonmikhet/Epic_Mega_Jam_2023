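; BP_Monument_2_Activator is a placeable interaction point that activates the second monument and opens its doors.
; On EventInteraction it destroys its Box component and swaps materials on the Monitor and StaticMesh.
; After short delays it reveals a Cylinder, then finds every BP_Monument2_Doors actor in the level and calls OpenDoors on each.
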(event `/Game/EpicMegaJam2023/Core/Interfaces/BPI_ItemInterface.EventInteraction`
  (params (Character :type "/Game/EpicMegaJam2023/Core/Character/MainCharacter/CH_MainCharacter Object Reference"))
  (`ActorComponent.K2_DestroyComponent` (`self.Box`))
  (`PrimitiveComponent.SetMaterial` (`self.Monitor`) 0 "/Game/EpicMegaJam2023/M_Beam.M_Beam")
  (`PrimitiveComponent.SetMaterial` (`self.StaticMesh`) 0 "/Game/EpicMegaJam2023/Art/M_Rocks.M_Rocks")
  (`KismetSystemLibrary.Delay` 1.0)
  (`SceneComponent.SetVisibility` (`self.Cylinder`) true false)
  (`KismetSystemLibrary.Delay` 1.0)
  (bind _outactors (`GameplayStatics.GetAllActorsOfClass` "/Game/EpicMegaJam2023/Core/Placeables/BP_Monument2_Doors.BP_Monument2_Doors_C"))
  (for _array_element _outactors
    (`/Game/EpicMegaJam2023/Core/Placeables/BP_Monument2_Doors.OpenDoors` _array_element)))

(fn `UserConstructionScript`
  (`parent.UserConstructionScript`))