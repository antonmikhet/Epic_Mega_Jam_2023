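; BP_LaserSensor_Platform is a placeable laser sensor variant whose triggered action rotates a platform a quarter turn.
; It caches the Scene component's relative transform on BeginPlay.
; The parent's StartAction is extended to destroy StaticMesh, then play a timeline that interpolates Scene to 90 degrees of added roll.
; Only forward playback is wired, with no reset.
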(event `self.ReceiveBeginPlay`
  (`parent.ReceiveBeginPlay`)
  (set `self.DefaultTransform` (`SceneComponent.GetRelativeTransform` (`self.Scene`))))

(event `self.StartAction`
  (bind _defaulttransform (`self.DefaultTransform`))
  (`parent.StartAction`)
  (`ActorComponent.K2_DestroyComponent` (`self.StaticMesh`))
  (bind (_direction _newtrack_0) (`Timeline|Timeline`)
    (:`Update`
      (`SceneComponent.K2_SetRelativeTransform` (`self.Scene`) (`KismetMathLibrary.TLerp` (`self.DefaultTransform`) (`KismetMathLibrary.MakeTransform` (.location _defaulttransform) (`KismetMathLibrary.MakeRotator` (+ (.roll (.rotation _defaulttransform)) 90.0) (.pitch (.rotation _defaulttransform)) (.yaw (.rotation _defaulttransform))) (.scale _defaulttransform)) _newtrack_0) false false))))

(fn `UserConstructionScript`
  (`parent.UserConstructionScript`))