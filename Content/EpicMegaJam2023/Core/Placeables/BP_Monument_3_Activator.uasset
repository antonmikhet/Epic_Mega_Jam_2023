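; Interactable activator for the third monument that lights it up and starts the game's final cutscene.
; It hides its Cylinder on BeginPlay; on interaction it destroys its Box, swaps the monitor and mesh materials, and reveals the Cylinder after a one-second delay.
; It then creates and plays a Level Sequence, binding a finish event that is currently empty.
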(event `self.ReceiveBeginPlay`
  (`parent.ReceiveBeginPlay`)
  (`SceneComponent.SetVisibility` (`self.Cylinder`) false false))

(event `/Game/EpicMegaJam2023/Core/Interfaces/BPI_ItemInterface.EventInteraction`
  (params (Character :type "/Game/EpicMegaJam2023/Core/Character/MainCharacter/CH_MainCharacter Object Reference"))
  (`ActorComponent.K2_DestroyComponent` (`self.Box`))
  (`PrimitiveComponent.SetMaterial` (`self.Monitor`) 0 "/Game/EpicMegaJam2023/Art/Material/M_Beam.M_Beam")
  (`PrimitiveComponent.SetMaterial` (`self.StaticMesh`) 0 "/Game/EpicMegaJam2023/Art/Material/M_Rocks.M_Rocks")
  (`KismetSystemLibrary.Delay` 1.0)
  (`SceneComponent.SetVisibility` (`self.Cylinder`) true false)
  (`self.StartFinalCutscene`))

(event `StartFinalCutscene`
  (bind _outactor (`LevelSequencePlayer.CreateLevelSequencePlayer` (`self.Level Sequence`) (`self.Settings`)))
  (bind _sequenceplayer (`LevelSequenceActor.SequencePlayer` _outactor))
  (`MovieSceneSequencePlayer.Play` _sequenceplayer)
  (add `MovieSceneSequencePlayer.OnFinished` _sequenceplayer (delegate `OnFinishedEvent`)))

(event `OnFinishedEvent`)

(fn `UserConstructionScript`
  (`parent.UserConstructionScript`))