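; BP_BasePickUpItem is the base pickup actor that the main character can collect as an item.
; Overlapping its box shows a prompt widget and registers it as the character's InteractionItem; leaving hides and clears it.
; On interaction it adds an ItemComponentClass component to the character, stores it in ItemsMap as the active item, then destroys itself.
; The construction script applies the configurable mesh and hides the widget.
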(event `self.Box.OnComponentBeginOverlap`
  (params (OverlappedComponent :type "PrimitiveComponent Object Reference") (OtherActor :type "Actor Object Reference") (OtherComp :type "PrimitiveComponent Object Reference") (OtherBodyIndex :type Integer) (bFromSweep :type Boolean) (SweepResult :type "HitResult Structure (by ref)"))
  (bind _asch_main_character (cast `/Game/EpicMegaJam2023/Core/Character/MainCharacter/CH_MainCharacter` OtherActor))
  (`SceneComponent.SetVisibility` (`self.Widget`) true false)
  (set `/Game/EpicMegaJam2023/Core/Character/MainCharacter/CH_MainCharacter.InteractionItem` self _asch_main_character))

(event `self.Box.OnComponentEndOverlap`
  (params (OverlappedComponent :type "PrimitiveComponent Object Reference") (OtherActor :type "Actor Object Reference") (OtherComp :type "PrimitiveComponent Object Reference") (OtherBodyIndex :type Integer))
  (bind _asch_main_character (cast `/Game/EpicMegaJam2023/Core/Character/MainCharacter/CH_MainCharacter` OtherActor))
  (`SceneComponent.SetVisibility` (`self.Widget`) false false)
  (set `/Game/EpicMegaJam2023/Core/Character/MainCharacter/CH_MainCharacter.InteractionItem` null _asch_main_character))

(event `/Game/EpicMegaJam2023/Core/Interfaces/BPI_ItemInterface.EventInteraction`
  (params (Character :type "/Game/EpicMegaJam2023/Core/Character/MainCharacter/CH_MainCharacter Object Reference"))
  (`/Engine/EditorBlueprintResources/StandardMacros.IsValid` Character
    (:`Is Valid`
      (bind _returnvalue (`|AddComponentByClass` Character (`self.ItemComponentClass`) (`self.Mesh`)))
      (bind _currentitem (`/Game/EpicMegaJam2023/Core/Components/AC_BaseItemComponent.CurrentItem` _returnvalue))
      (`BlueprintMapLibrary.Map_Add` (`/Game/EpicMegaJam2023/Core/Character/MainCharacter/CH_MainCharacter.ItemsMap` Character) _currentitem _returnvalue)
      (set `/Game/EpicMegaJam2023/Core/Character/MainCharacter/CH_MainCharacter.CurrentActiveItem` _currentitem Character)
      (`self.K2_DestroyActor`))))

(fn `UserConstructionScript`
  (`StaticMeshComponent.SetStaticMesh` (`self.StaticMesh`) (`self.Mesh`))
  (`SceneComponent.SetVisibility` (`self.Widget`) false false))