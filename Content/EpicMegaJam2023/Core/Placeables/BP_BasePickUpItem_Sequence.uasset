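; A placeable pickup item Blueprint that plays a Level Sequence when interacted with.
; EventInteraction creates a sequence player from the LevelSequence and Settings variables, starts playback, then binds OnFinishedEvent to the player's finished delegate.
; OnFinishedEvent is empty, and the construction script only calls its parent.
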(event `/Game/EpicMegaJam2023/Core/Interfaces/BPI_ItemInterface.EventInteraction`
  (params (Character :type "/Game/EpicMegaJam2023/Core/Character/MainCharacter/CH_MainCharacter Object Reference"))
  (bind _outactor (`LevelSequencePlayer.CreateLevelSequencePlayer` (`self.Level Sequence`) (`self.Settings`)))
  (bind _sequenceplayer (`LevelSequenceActor.SequencePlayer` _outactor))
  (`MovieSceneSequencePlayer.Play` _sequenceplayer)
  (add `MovieSceneSequencePlayer.OnFinished` _sequenceplayer (delegate `OnFinishedEvent`)))

(event `OnFinishedEvent`)

(fn `UserConstructionScript`
  (`parent.UserConstructionScript`))