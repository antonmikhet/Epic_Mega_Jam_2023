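; BP_LastMessage_Activator is an interactable console button that triggers the game's final screen.
; On interaction it changes the character's input state, fires the checkpoint component's kill event, plays a click, destroys its box and swaps console and button materials.
; After a short delay it shows WB_FinalScreen and stores it as the character's InteractionItem.
; A level-sequence cutscene path exists but is unconnected; StartFinalCutscene is empty.
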(event `self.ReceiveBeginPlay`
  (`parent.ReceiveBeginPlay`))

(event `/Game/EpicMegaJam2023/Core/Interfaces/BPI_ItemInterface.EventInteraction`
  (params (Character :type "/Game/EpicMegaJam2023/Core/Character/MainCharacter/CH_MainCharacter Object Reference"))
  (bind _output_get (set `self.Character` Character))
  (`/Game/EpicMegaJam2023/Core/Character/MainCharacter/CH_MainCharacter.SetInputStates` _output_get "NewEnumerator2")
  (`/Game/EpicMegaJam2023/Core/Components/AC_CheckPointSystem.OnEventKill` (`self.GetComponentByClass` _output_get "/Game/EpicMegaJam2023/Core/Components/AC_CheckPointSystem.AC_CheckPointSystem_C"))
  (`GameplayStatics.PlaySound2D` "/Game/EpicMegaJam2023/Core/Audio/Metasounds/MS_Button.MS_Button" 1.0 1.0 0.0 null null)
  (`ActorComponent.K2_DestroyComponent` (`self.Box`))
  (`PrimitiveComponent.SetMaterial` (`self.Console`) 1 "/Game/EpicMegaJam2023/Art/Material/M_Beam.M_Beam")
  (`PrimitiveComponent.SetMaterial` (`self.Button`) 0 "/Game/EpicMegaJam2023/Art/Material/M_Rocks.M_Rocks")
  (`KismetSystemLibrary.Delay` 0.5)
  (bind _returnvalue (`|GenericCreateObject` "/Game/EpicMegaJam2023/Core/UI/FinalScreen/WB_FinalScreen.WB_FinalScreen_C"))
  (`UserWidget.AddToViewport` _returnvalue 0)
  (set `/Game/EpicMegaJam2023/Core/Character/MainCharacter/CH_MainCharacter.InteractionItem` _returnvalue (`self.Character`)))

(event `StartFinalCutscene`)

(event `OnFinishedEvent`
  (`KismetSystemLibrary.PrintString` "EVENT FINISHED")
  (`/Game/EpicMegaJam2023/Core/Character/MainCharacter/CH_MainCharacter.SetInputStates` (`self.Character`) "NewEnumerator0"))

(fn `UserConstructionScript`
  (`parent.UserConstructionScript`))