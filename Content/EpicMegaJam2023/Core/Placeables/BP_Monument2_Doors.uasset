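; Placeable double-door actor for a monument that slides open when its OpenDoors event is called.
; BeginPlay caches both doors' relative transforms, then OpenDoors plays a door sound and runs a Timeline that lerps each door apart along local X.
; The right door's target is built from the left door's cached transform rather than its own.
; There is no closing logic.
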(event `self.ReceiveBeginPlay`
  (`parent.ReceiveBeginPlay`)
  (set `self.DefaultTransformLeftDoor` (`SceneComponent.GetRelativeTransform` (`self.Scene_Left`)))
  (set `self.DefaultTransformRightDoor` (`SceneComponent.GetRelativeTransform` (`self.Scene_Right`))))

(event `OpenDoors`
  (bind _defaulttransformleftdoor (`self.DefaultTransformLeftDoor`))
  (bind _defaulttransformleftdoor_2 (`self.DefaultTransformLeftDoor`))
  (`GameplayStatics.PlaySoundAtLocation` "/Game/EpicMegaJam2023/Core/Audio/Metasounds/MS_Doors.MS_Doors" (`SceneComponent.K2_GetComponentLocation` (`self.Root`)) (struct) 1.0 1.0 0.0 null null null null)
  (bind (_direction _newtrack_0) (`Timeline|Timeline`)
    (:`Update`
      (`SceneComponent.K2_SetRelativeTransform` (`self.Scene_Left`) (`KismetMathLibrary.TLerp` (`self.DefaultTransformLeftDoor`) (`KismetMathLibrary.MakeTransform` (`KismetMathLibrary.MakeVector` (+ (.x (.location _defaulttransformleftdoor)) -150.0) (.y (.location _defaulttransformleftdoor)) (.z (.location _defaulttransformleftdoor))) (.rotation _defaulttransformleftdoor) (.scale _defaulttransformleftdoor)) _newtrack_0) false false)
      (`SceneComponent.K2_SetRelativeTransform` (`self.Scene_Right`) (`KismetMathLibrary.TLerp` (`self.DefaultTransformRightDoor`) (`KismetMathLibrary.MakeTransform` (`KismetMathLibrary.MakeVector` (+ (.x (.location _defaulttransformleftdoor_2)) 150.0) (.y (.location _defaulttransformleftdoor_2)) (.z (.location _defaulttransformleftdoor_2))) (.rotation _defaulttransformleftdoor_2) (.scale _defaulttransformleftdoor_2)) _newtrack_0) false false))))

(fn `UserConstructionScript`
  (`parent.UserConstructionScript`))