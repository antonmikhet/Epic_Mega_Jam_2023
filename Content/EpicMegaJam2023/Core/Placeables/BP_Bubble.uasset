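; BP_Bubble is a placeable bubble hazard that floats, homes in on the player character and bursts on contact, dealing damage.
; BubbleManager events drive bobbing and scale pulsing instead of Tick, with randomized settings and a timeline spawn grow-in.
; An outer magnet sphere starts a looping chase timer, bound to the checkpoint component's kill event.
; Contact, optional lifetime expiry or ToggleState triggers DestroyBubble, briefly running a timer before destroying the actor.
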(event `self.ReceiveBeginPlay`
  (bind _output (`|ConvertAsset` (`self.BubbleManager`)))
  (`|ExecutionSequence`
    (:`then_0`
      (`self.SetDefaultSettings`))
    (:`then_1`
      (if (`self.IsAlive`)
        (if (`self.InfiniteLife`)
          (add `/Game/EpicMegaJam2023/Core/Placeables/BP_BubbleManager.OnBubbleChangeSign` _output (delegate `MoveEvent`) :!label _label)
          (add `/Game/EpicMegaJam2023/Core/Placeables/BP_BubbleManager.OnBubbleTick` _output (delegate `MoveTick`))
          (else
            (`|ExecutionSequence`
              (:`then_0`
                (goto _label))
              (:`then_1`
                (bind _returnvalue (`KismetSystemLibrary.K2_SetTimerDelegate` (delegate `DestrpyAfterTimer`) (`KismetMathLibrary.RandomFloatInRange` 7.0 20.0)))))))))
    (:`then_2`
      (`SceneComponent.SetWorldScale3D` (`self.Scene`) (0.0 0.0 0.0))
      (bind (_direction _alpha) (`Timeline|SpawnTimeline` :!via `PlayFromStart`)
        (:`Update`
          (`SceneComponent.SetWorldScale3D` (`self.Scene`) (`KismetMathLibrary.VLerp` (0.0 0.0 0.0) (`self.StartScale`) _alpha)))))))

(event `DestrpyAfterTimer`
  (`KismetSystemLibrary.K2_ClearAndInvalidateTimerHandle` (stale `self.ReceiveBeginPlay` _returnvalue))
  (`self.DestroyBubble`))

(event `MoveEvent`
  (set `self.Sign` (* (`self.Sign`) -1.0)))

(event `MoveTick`
  (`self.K2_AddActorLocalOffset` (- (`self.K2_GetActorLocation`) (+ (`self.K2_GetActorLocation`) (`KismetMathLibrary.MakeVector` 0.0 0.0 (* (`self.Sign`) (`self.FloatingRangeZ`))))))
  (`SceneComponent.SetWorldScale3D` (`self.Scene`) (+ (* (`self.ScaleTickDelta`) (`self.Sign`)) (`self.GetActorScale3D`))))

(event `self.Sphere.OnComponentBeginOverlap`
  (params (OverlappedComponent :type "PrimitiveComponent Object Reference") (OtherActor :type "Actor Object Reference") (OtherComp :type "PrimitiveComponent Object Reference") (OtherBodyIndex :type Integer) (bFromSweep :type Boolean) (SweepResult :type "HitResult Structure (by ref)"))
  (bind _asch_main_character (cast `/Game/EpicMegaJam2023/Core/Character/MainCharacter/CH_MainCharacter` OtherActor))
  (`self.DestroyBubble`)
  (`/Engine/EditorBlueprintResources/StandardMacros.DoOnce` false
    (:`Completed`
      (`GameplayStatics.ApplyDamage` _asch_main_character (`self.Base Damage`)))))

(event `DestroyBubble`
  (set `self.IsAlive` false)
  (bind _returnvalue (`KismetSystemLibrary.K2_SetTimerDelegate` (`|CreateDelegate` :!event `ScaleBubbleDestroy`) 0.01 true))
  (`KismetSystemLibrary.Delay` 0.15)
  (`KismetSystemLibrary.K2_ClearAndInvalidateTimerHandle` _returnvalue)
  (`self.K2_DestroyActor`))

(event `/Game/EpicMegaJam2023/Core/Interfaces/BPI_LaserInterface.ToggleState`
  (params (`On/Off` :type Boolean))
  (if `On/Off`
    (`/Engine/EditorBlueprintResources/StandardMacros.DoOnce` false
      (:`Completed`
        (`self.DestroyBubble`)))))

(event `self.SphereMagnit.OnComponentBeginOverlap`
  (params (OverlappedComponent :type "PrimitiveComponent Object Reference") (OtherActor :type "Actor Object Reference") (OtherComp :type "PrimitiveComponent Object Reference") (OtherBodyIndex :type Integer) (bFromSweep :type Boolean) (SweepResult :type "HitResult Structure (by ref)"))
  (bind _asch_main_character (cast `/Game/EpicMegaJam2023/Core/Character/MainCharacter/CH_MainCharacter` OtherActor))
  (bind _output_get (set `self.As CH Main Character` _asch_main_character))
  (add `/Game/EpicMegaJam2023/Core/Components/AC_CheckPointSystem.OnEventKill` (`self.GetComponentByClass` _output_get "/Game/EpicMegaJam2023/Core/Components/AC_CheckPointSystem.AC_CheckPointSystem_C") (`|CreateDelegate` :!event `OnCharacterKilled`))
  (bind _returnvalue (`KismetSystemLibrary.K2_SetTimerDelegate` (`|CreateDelegate` :!event `EvetTimerMove`) 0.01 true))
  (set `self.MoveTImer` _returnvalue))

(event `EvetTimerMove`
  (if (and (`KismetSystemLibrary.IsValid` self) (`KismetSystemLibrary.IsValid` (`self.As CH Main Character`)))
    (`self.K2_SetActorLocation` (+ (`KismetMathLibrary.GetDirectionUnitVector` (`self.K2_GetActorLocation`) (+ (`self.K2_GetActorLocation` (`self.As CH Main Character`)) (`KismetMathLibrary.MakeVector` 0.0 0.0 (`CapsuleComponent.GetScaledCapsuleHalfHeight` (`Character.CapsuleComponent` (`self.As CH Main Character`)))))) (`self.K2_GetActorLocation`)))))

(fn `OnCharacterKilled`
  (`KismetSystemLibrary.K2_ClearAndInvalidateTimerHandle` (`self.MoveTImer`)))

(fn `ScaleBubbleDestroy`
  (bind _dynamicmaterialinstance (`self.DynamicMaterialInstance`))
  (`SceneComponent.SetWorldScale3D` (`self.StaticMesh`) (+ (`SceneComponent.K2_GetComponentScale` (`self.StaticMesh`)) (0.015 0.015 0.015)))
  (bind _returnvalue (`MaterialInstanceDynamic.K2_GetVectorParameterValue` _dynamicmaterialinstance "EmissiveColor"))
  (`MaterialInstanceDynamic.SetVectorParameterValue` _dynamicmaterialinstance "EmissiveColor" (`KismetMathLibrary.MakeColor` (+ (`.R` (break `LinearColor` _returnvalue)) 0.01)))
  (`GameplayStatics.PlayWorldCameraShake` (`self.CameraShakeClass`) (`self.K2_GetActorLocation`) (`self.Inner Radius`) (`self.Outer Radius`) (`self.Falloff`)))

(fn `SetDefaultSettings`
  (set `self.Sign` (select `int` (`KismetMathLibrary.RandomInteger` 5) :`0` -1.0 :`1` 1.0 :`2` -1.0 :`3` 1.0 :`4` -1.0 :`5` 1.0))
  (set `self.StartScale` (`KismetMathLibrary.Conv_DoubleToVector` (`KismetMathLibrary.RandomFloatInRange` 0.2 1.0)))
  (`SceneComponent.SetRelativeScale3D` (`self.Scene`) (`self.StartScale`))
  (set `self.ScaleTickDelta` (`KismetMathLibrary.Conv_DoubleToVector` (`KismetMathLibrary.RandomFloatInRange` 0.0005 0.0015)))
  (set `self.FloatingRangeZ` (`KismetMathLibrary.RandomFloatInRange` 1.0 1.6))
  (bind _returnvalue (`PrimitiveComponent.CreateDynamicMaterialInstance` (`self.StaticMesh`) 0 (`PrimitiveComponent.GetMaterial` (`self.StaticMesh`) 0) "None"))
  (set `self.DynamicMaterialInstance` _returnvalue))

(fn `UserConstructionScript`
  (`SphereComponent.SetSphereRadius` (`self.SphereMagnit`) (`self.InteractionRaduisSphere Radius`) true))