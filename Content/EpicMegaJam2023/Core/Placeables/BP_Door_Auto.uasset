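; Automatic sliding double door that opens when the main character enters its box trigger and closes when they leave.
; BeginPlay removes a static mesh and caches both door scene components' relative transforms.
; Overlap events play or reverse a Timeline that lerps the halves apart along local X.
; The right door's open target is derived from the left door's default transform, not its own.
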(event `self.ReceiveBeginPlay`
  (`parent.ReceiveBeginPlay`)
  (`ActorComponent.K2_DestroyComponent` (`self.StaticMesh`))
  (set `self.DefaultTransformLeftDoor` (`SceneComponent.GetRelativeTransform` (`self.Scene_Left`)))
  (set `self.DefaultTransformRightDoor` (`SceneComponent.GetRelativeTransform` (`self.Scene_Right`))))

(event `self.Box.OnComponentBeginOverlap`
  (params (OverlappedComponent :type "PrimitiveComponent Object Reference") (OtherActor :type "Actor Object Reference") (OtherComp :type "PrimitiveComponent Object Reference") (OtherBodyIndex :type Integer) (bFromSweep :type Boolean) (SweepResult :type "HitResult Structure (by ref)"))
  (bind _defaulttransformleftdoor (`self.DefaultTransformLeftDoor`))
  (bind _defaulttransformleftdoor_2 (`self.DefaultTransformLeftDoor`))
  (cast `/Game/EpicMegaJam2023/Core/Character/MainCharacter/CH_MainCharacter` OtherActor)
  (bind (_direction _newtrack_0) (`Timeline|Timeline` :!label _label)
    (:`Update`
      (`SceneComponent.K2_SetRelativeTransform` (`self.Scene_Left`) (`KismetMathLibrary.TLerp` (`self.DefaultTransformLeftDoor`) (`KismetMathLibrary.MakeTransform` (`KismetMathLibrary.MakeVector` (+ (.x (.location _defaulttransformleftdoor)) -150.0) (.y (.location _defaulttransformleftdoor)) (.z (.location _defaulttransformleftdoor))) (.rotation _defaulttransformleftdoor) (.scale _defaulttransformleftdoor)) _newtrack_0) false false)
      (`SceneComponent.K2_SetRelativeTransform` (`self.Scene_Right`) (`KismetMathLibrary.TLerp` (`self.DefaultTransformRightDoor`) (`KismetMathLibrary.MakeTransform` (`KismetMathLibrary.MakeVector` (+ (.x (.location _defaulttransformleftdoor_2)) 150.0) (.y (.location _defaulttransformleftdoor_2)) (.z (.location _defaulttransformleftdoor_2))) (.rotation _defaulttransformleftdoor_2) (.scale _defaulttransformleftdoor_2)) _newtrack_0) false false))))

(event `self.Box.OnComponentEndOverlap`
  (params (OverlappedComponent :type "PrimitiveComponent Object Reference") (OtherActor :type "Actor Object Reference") (OtherComp :type "PrimitiveComponent Object Reference") (OtherBodyIndex :type Integer))
  (cast `/Game/EpicMegaJam2023/Core/Character/MainCharacter/CH_MainCharacter` OtherActor)
  (goto _label :!via `Reverse`))

(fn `UserConstructionScript`
  (`parent.UserConstructionScript`))