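; BP_LaserSensor_Sequence is a laser sensor placeable that plays a Level Sequence when its action starts.
; StartAction runs the parent logic, destroys the sensor's static mesh, then creates a sequence player for the configured LevelSequence and plays it.
; A handler is bound to the player's finished event but does nothing yet.
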(event `self.ReceiveBeginPlay`
  (`parent.ReceiveBeginPlay`))

(event `self.StartAction`
  (`parent.StartAction`)
  (`ActorComponent.K2_DestroyComponent` (`self.StaticMesh`))
  (bind _outactor (`LevelSequencePlayer.CreateLevelSequencePlayer` (`self.Level Sequence`) (`self.Settings`)))
  (bind _sequenceplayer (`LevelSequenceActor.SequencePlayer` _outactor))
  (`MovieSceneSequencePlayer.Play` _sequenceplayer)
  (add `MovieSceneSequencePlayer.OnFinished` _sequenceplayer (delegate `OnFinished_Event`)))

(event `OnFinished_Event`)

(fn `UserConstructionScript`
  (`parent.UserConstructionScript`))