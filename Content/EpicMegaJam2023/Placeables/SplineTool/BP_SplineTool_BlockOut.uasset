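; Spline placement tool for blocking out levels that fills a spline with meshes defined by an ObjectList.
; Construction or RebuildSpline clears tracked components, then GenerateSpline places each entry as stretched spline meshes, length-based segments, instances or static meshes.
; Helpers pick meshes by default, random or sequence, derive spacing from bounds or gap, and supply seeded random transforms.
; DropSpline traces points onto the ground, optionally aligning up vectors, and rebuilds.
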(event `RebuildSpline`
  (`self.BuildSpline`))

(event `DropSpline`
  (for _index (range (`SplineComponent.GetNumberOfSplinePoints` (`self.Spline`)))
    (bind _returnvalue (`SplineComponent.GetLocationAtSplinePoint` (`self.Spline`) _index "World"))
    (bind (_outhit _returnvalue_2) (`KismetSystemLibrary.LineTraceSingleForObjects` (+ _returnvalue (0.0 0.0 200.0)) (- _returnvalue (0.0 0.0 1000.0)) (`self.DropSplineCollisionCheck`)))
    (if _returnvalue_2
      (bind (_bblockinghit _binitialoverlap _time _distance _location _impactpoint _normal) (`GameplayStatics.BreakHitResult` _outhit))
      (`SplineComponent.SetLocationAtSplinePoint` (`self.Spline`) _index _location "World" true)
      (if (`self.SnapToGroundAngle`)
        (`SplineComponent.SetUpVectorAtSplinePoint` (`self.Spline`) _index _normal "World" true))))
  (`self.BuildSpline`))

(fn `BuildSpline`
  (`self.Clear Spline Meshes`)
  (for (_array_element _array_index) (`self.ObjectList`)
    (set `self.ArrayElement` _array_element)
    (set `self.ArrayIndex` _array_index)
    (`self.GenerateSpline`)))

(fn `Clear Spline Meshes`
  (`|ExecutionSequence`
    (:`then_0`
      (for _array_element (`self.MeshesArray`)
        (`ActorComponent.K2_DestroyComponent` _array_element))
      (`KismetArrayLibrary.Array_Clear` (`self.MeshesArray`)))
    (:`then_1`
      (for _array_element_2 (`self.StaticMeshComponentArray`)
        (`ActorComponent.K2_DestroyComponent` _array_element_2))
      (`KismetArrayLibrary.Array_Clear` (`self.StaticMeshComponentArray`)))))

(fn `GenerateSpline`
  (bind (_returnlocation _returnrotation _returnscale) (`self.GetRandom`))
  (bind (_returnlocation_2 _returnrotation_2 _returnscale_2) (`self.GetRandom`))
  (bind (_randomrotationvalue_roll _randomrotationvalue_pitch _randomrotationvalue_yaw) (`KismetMathLibrary.BreakRotator` (`self.RandomRotationValue`)))
  (bind (_randomrotationvalue_roll_2 _randomrotationvalue_pitch_2 _randomrotationvalue_yaw_2) (`KismetMathLibrary.BreakRotator` (`self.RandomRotationValue`)))
  (bind _spline (`self.Spline`))
  (bind _meshscale (`self.MeshScale`))
  (bind _spline_2 (`self.Spline`))
  (bind _spline_3 (`self.Spline`))
  (bind _meshscale_2 (`self.MeshScale`))
  (bind _spline_4 (`self.Spline`))
  (bind ((`MainParameters_28_05803D8A4D7C13045734EB9AF7605BC4` _mainparameters) (`RandomParameters_34_758F8DA4491FFE18494D49ABA5B57785` _randomparameters)) (break `/Game/EpicMegaJam2023/Placeables/SplineTool/Structures/S_SplineTool_ObjectList` (`self.ArrayElement`)))
  (bind ((`MainParameters_28_05803D8A4D7C13045734EB9AF7605BC4` _mainparameters_2) (`RandomParameters_34_758F8DA4491FFE18494D49ABA5B57785` _randomparameters_2)) (break `/Game/EpicMegaJam2023/Placeables/SplineTool/Structures/S_SplineTool_ObjectList` (`self.ArrayElement`)))
  (bind _returnvalue (* (`self.SplineIndex`) (`self.GetLength`)))
  (bind _returnvalue_2 (- (`self.SplineIndex`) 1))
  (bind _returnvalue_3 (+ (`self.SplineIndex`) 1))
  (bind _returnvalue_4 (`SplineComponent.GetLocationAtDistanceAlongSpline` (`self.Spline`) (* (`self.SplineIndex`) (`self.GetLength`)) "Local"))
  (bind _returnvalue_5 (`SplineComponent.GetLocationAtDistanceAlongSpline` (`self.Spline`) (* (`self.SplineIndex`) (`self.GetLength`)) "World"))
  (bind _returnvalue_6 (* (+ (`self.SplineIndex`) 1) (`self.GetLength`)))
  (bind _outinstancetransform (`InstancedStaticMeshComponent.GetInstanceTransform` (`self.InstancedStaticMesh`) _returnvalue_2 true))
  (bind _y (.y (.location (`.OffsetTransform_16_E65CCBA647A306B6467796A17ED42FDE` (break `/Game/EpicMegaJam2023/Placeables/SplineTool/Structures/S_SplineTool_MainParameters` (`.MainParameters_28_05803D8A4D7C13045734EB9AF7605BC4` (break `/Game/EpicMegaJam2023/Placeables/SplineTool/Structures/S_SplineTool_ObjectList` (`self.ArrayElement`))))))))
  (bind _z (.z (.location (`.OffsetTransform_16_E65CCBA647A306B6467796A17ED42FDE` (break `/Game/EpicMegaJam2023/Placeables/SplineTool/Structures/S_SplineTool_MainParameters` (`.MainParameters_28_05803D8A4D7C13045734EB9AF7605BC4` (break `/Game/EpicMegaJam2023/Placeables/SplineTool/Structures/S_SplineTool_ObjectList` (`self.ArrayElement`))))))))
  (bind _y_2 (.y (.location (`.OffsetTransform_16_E65CCBA647A306B6467796A17ED42FDE` (break `/Game/EpicMegaJam2023/Placeables/SplineTool/Structures/S_SplineTool_MainParameters` (`.MainParameters_28_05803D8A4D7C13045734EB9AF7605BC4` (break `/Game/EpicMegaJam2023/Placeables/SplineTool/Structures/S_SplineTool_ObjectList` (`self.ArrayElement`))))))))
  (bind _z_2 (.z (.location (`.OffsetTransform_16_E65CCBA647A306B6467796A17ED42FDE` (break `/Game/EpicMegaJam2023/Placeables/SplineTool/Structures/S_SplineTool_MainParameters` (`.MainParameters_28_05803D8A4D7C13045734EB9AF7605BC4` (break `/Game/EpicMegaJam2023/Placeables/SplineTool/Structures/S_SplineTool_ObjectList` (`self.ArrayElement`))))))))
  (if (`KismetArrayLibrary.Array_IsValidIndex` (`.StaticMesh_30_459BCB424BFD738D8803C588166C39B6` (break `/Game/EpicMegaJam2023/Placeables/SplineTool/Structures/S_SplineTool_ObjectList` (`self.ArrayElement`))))
    (set `self.SequenceIndex` 0)
    (switch `/Game/EpicMegaJam2023/Placeables/SplineTool/Enumerators/E_SplineTool_ObjectTypes` (`.PlacementType_29_4B76077C42C7C4CD7111EEA7B93C61DB` (break `/Game/EpicMegaJam2023/Placeables/SplineTool/Structures/S_SplineTool_ObjectList` (`self.ArrayElement`)))
      (:`NewEnumerator0`
        ;[1 1 1] Stretched
        (for _index (range (+ (- (`SplineComponent.GetNumberOfSplinePoints` (`self.Spline`)) 2) 1))
          (set `self.SplineIndex` _index)
          (bind _returnvalue_7 (`AddComponent|NODE_AddSplineMeshComponent-3` :`RelativeTransform` (`KismetMathLibrary.MakeTransform` (0.0 0.0 0.0) (struct) (.scale (`.OffsetTransform_16_E65CCBA647A306B6467796A17ED42FDE` (break `/Game/EpicMegaJam2023/Placeables/SplineTool/Structures/S_SplineTool_MainParameters` (`.MainParameters_28_05803D8A4D7C13045734EB9AF7605BC4` (break `/Game/EpicMegaJam2023/Placeables/SplineTool/Structures/S_SplineTool_ObjectList` (`self.ArrayElement`)))))))))
          (bind _output_get (set `self.SplineMeshCompontn` _returnvalue_7))
          (`KismetArrayLibrary.Array_Add` (`self.MeshesArray`) _output_get)
          (`StaticMeshComponent.SetStaticMesh` _output_get (`self.GetMesh`))
          (`SplineMeshComponent.SetStartAndEnd` (`self.SplineMeshCompontn`) (`SplineComponent.GetLocationAtSplinePoint` _spline_4 (`self.SplineIndex`) "Local") (`SplineComponent.GetTangentAtSplinePoint` _spline_4 0 "Local") (`SplineComponent.GetLocationAtSplinePoint` _spline_3 _returnvalue_3 "Local") (`SplineComponent.GetTangentAtSplinePoint` _spline_3 _returnvalue_3 "Local") true)
          (`SplineMeshComponent.SetStartOffset` (`self.SplineMeshCompontn`) (`KismetMathLibrary.MakeVector2D` _y_2 _z_2) true)
          (`SplineMeshComponent.SetEndOffset` (`self.SplineMeshCompontn`) (`KismetMathLibrary.MakeVector2D` _y_2 _z_2) true)
          (`PrimitiveComponent.SetCollisionEnabled` (`self.SplineMeshCompontn`) (`self.CollisionEnabled`))
          (bind _physicsmaterial (`self.PhysicsMaterial`)
            (:`then`
              (`PrimitiveComponent.SetPhysMaterialOverride` (`self.SplineMeshCompontn`) _physicsmaterial))
            (:`else`
              _))
          (`PrimitiveComponent.SetRenderCustomDepth` (`self.SplineMeshCompontn`) (`self.CustomDepth`))
          (`PrimitiveComponent.SetCastShadow` (`self.SplineMeshCompontn`) (`self.CastShadow`))))
      (:`NewEnumerator3`
        ;[1 1 1] Segments
        (for _index_2 (range (+ (`KismetMathLibrary.FTrunc` (/ (`SplineComponent.GetSplineLength` (`self.Spline`)) (`self.GetLength`))) 1))
          (set `self.SplineIndex` _index_2)
          (bind _returnvalue_8 (`AddComponent|NODE_AddSplineMeshComponent-4`))
          (bind _output_get_2 (set `self.SplineMeshCompontn` _returnvalue_8))
          (`StaticMeshComponent.SetStaticMesh` _output_get_2 (`self.GetMesh`))
          (`KismetArrayLibrary.Array_Add` (`self.MeshesArray`) _output_get_2)
          (`SplineMeshComponent.SetStartAndEnd` (`self.SplineMeshCompontn`) (`SplineComponent.GetLocationAtDistanceAlongSpline` _spline_2 _returnvalue "Local") (`KismetMathLibrary.ClampVectorSize` (`SplineComponent.GetTangentAtDistanceAlongSpline` _spline_2 _returnvalue "Local") 0.0 (`self.GetLength`)) (`SplineComponent.GetLocationAtDistanceAlongSpline` _spline _returnvalue_6 "Local") (`KismetMathLibrary.ClampVectorSize` (`SplineComponent.GetTangentAtDistanceAlongSpline` _spline _returnvalue_6 "Local") 0.0 (`self.GetLength`)) true)
          (`SplineMeshComponent.SetStartOffset` (`self.SplineMeshCompontn`) (`KismetMathLibrary.MakeVector2D` _y _z) true)
          (`SplineMeshComponent.SetEndOffset` (`self.SplineMeshCompontn`) (`KismetMathLibrary.MakeVector2D` _y _z) true)
          (`SplineMeshComponent.SetStartScale` (`self.SplineMeshCompontn`) (`KismetMathLibrary.MakeVector2D` _meshscale_2 _meshscale_2) true)
          (`SplineMeshComponent.SetEndScale` (`self.SplineMeshCompontn`) (`KismetMathLibrary.MakeVector2D` _meshscale _meshscale) true)
          (if (`.Enable_24_E4159E5743B0C57C691F6BA06D527D29` (break `/Game/EpicMegaJam2023/Placeables/SplineTool/Structures/S_SplineTool_RandomRotationOffset` (`.RandomRotation_38_D77C9F92438796B4C97AD6ACD9B9F1A7` (break `/Game/EpicMegaJam2023/Placeables/SplineTool/Structures/S_SplineTool_Random` (`.RandomParameters_34_758F8DA4491FFE18494D49ABA5B57785` (break `/Game/EpicMegaJam2023/Placeables/SplineTool/Structures/S_SplineTool_ObjectList` (`self.ArrayElement`)))))))
            (set `self.RandomRotationValue` (`.ReturnRotation` (`self.GetRandom`)))
            (`SplineMeshComponent.SetStartRoll` (`self.SplineMeshCompontn`) _randomrotationvalue_yaw_2 true)
            (`SplineMeshComponent.SetEndRoll` (`self.SplineMeshCompontn`) _randomrotationvalue_yaw true))
          (`PrimitiveComponent.SetCollisionEnabled` (`self.SplineMeshCompontn`) (`self.CollisionEnabled`))
          (bind _physicsmaterial_2 (`self.PhysicsMaterial`)
            (:`then`
              (`PrimitiveComponent.SetPhysMaterialOverride` (`self.SplineMeshCompontn`) _physicsmaterial_2))
            (:`else`
              _))
          (`PrimitiveComponent.SetRenderCustomDepth` (`self.SplineMeshCompontn`) (`self.CustomDepth`))
          (`PrimitiveComponent.SetCastShadow` (`self.SplineMeshCompontn`) (`self.CastShadow`))))
      (:`NewEnumerator1`
        ;[1 1 1] Instance
        (bind _returnvalue_9 (`AddComponent|NODE_AddInstancedStaticMeshComponent-2`))
        (set `self.InstancedStaticMesh` _returnvalue_9)
        (for _index_3 (range (+ (`KismetMathLibrary.FFloor` (/ (`SplineComponent.GetSplineLength` (`self.Spline`)) (`self.GetLength`))) 1))
          (set `self.SplineIndex` _index_3)
          (`StaticMeshComponent.SetStaticMesh` (`self.InstancedStaticMesh`) (`self.GetMesh`))
          (`InstancedStaticMeshComponent.AddInstanceWorldSpace` (`self.InstancedStaticMesh`) (`KismetMathLibrary.MakeTransform` (+ _returnvalue_5 (.location (`.OffsetTransform_16_E65CCBA647A306B6467796A17ED42FDE` (break `/Game/EpicMegaJam2023/Placeables/SplineTool/Structures/S_SplineTool_MainParameters` (`.MainParameters_28_05803D8A4D7C13045734EB9AF7605BC4` (break `/Game/EpicMegaJam2023/Placeables/SplineTool/Structures/S_SplineTool_ObjectList` (`self.ArrayElement`)))))))))
          (`InstancedStaticMeshComponent.UpdateInstanceTransform` (`self.InstancedStaticMesh`) _returnvalue_2 (`KismetMathLibrary.MakeTransform` (+ (.location _outinstancetransform) _returnlocation_2) (select `bool` (`.Enable_24_E4159E5743B0C57C691F6BA06D527D29` (break `/Game/EpicMegaJam2023/Placeables/SplineTool/Structures/S_SplineTool_RandomRotationOffset` (`.RandomRotation_38_D77C9F92438796B4C97AD6ACD9B9F1A7` (break `/Game/EpicMegaJam2023/Placeables/SplineTool/Structures/S_SplineTool_Random` _randomparameters)))) :`false` (select `bool` (`.RotateInstanceTowardsSpline_24_8CDE40054FEF3D3044EC138C725F4795` (break `/Game/EpicMegaJam2023/Placeables/SplineTool/Structures/S_SplineTool_MainParameters` _mainparameters)) :`false` (.rotation _outinstancetransform) :`true` (`KismetMathLibrary.FindLookAtRotation` (.location _outinstancetransform) _returnvalue_5)) :`true` _returnrotation_2) _returnscale_2) true false true)
          (`PrimitiveComponent.SetCollisionEnabled` (`self.InstancedStaticMesh`) (`self.CollisionEnabled`))
          (bind _physicsmaterial_3 (`self.PhysicsMaterial`)
            (:`then`
              (`PrimitiveComponent.SetPhysMaterialOverride` (`self.InstancedStaticMesh`) _physicsmaterial_3))
            (:`else`
              _))
          (`PrimitiveComponent.SetRenderCustomDepth` (`self.InstancedStaticMesh`) (`self.CustomDepth`))
          (`PrimitiveComponent.SetCastShadow` (`self.InstancedStaticMesh`) (`self.CastShadow`))))
      (:`NewEnumerator4`
        ;[1 1 1] StaticMeshes
        (for _index_4 (range (+ (`KismetMathLibrary.FFloor` (/ (`SplineComponent.GetSplineLength` (`self.Spline`)) (`self.GetLength`))) 1))
          (set `self.SplineIndex` _index_4)
          (bind _returnvalue_10 (`AddComponent|NODE_AddStaticMeshComponent-0` :`RelativeTransform` (`KismetMathLibrary.MakeTransform` (+ _returnlocation _returnvalue_4) (select `bool` (`.RotateInstanceTowardsSpline_24_8CDE40054FEF3D3044EC138C725F4795` (break `/Game/EpicMegaJam2023/Placeables/SplineTool/Structures/S_SplineTool_MainParameters` _mainparameters_2)) :`false` (select `bool` (`.Enable_24_E4159E5743B0C57C691F6BA06D527D29` (break `/Game/EpicMegaJam2023/Placeables/SplineTool/Structures/S_SplineTool_RandomRotationOffset` (`.RandomRotation_38_D77C9F92438796B4C97AD6ACD9B9F1A7` (break `/Game/EpicMegaJam2023/Placeables/SplineTool/Structures/S_SplineTool_Random` _randomparameters_2)))) :`true` _returnrotation) :`true` (`KismetMathLibrary.FindLookAtRotation` _returnvalue_4 (`self.K2_GetActorLocation`))) _returnscale)))
          (set `self.StaticMeshComponent` _returnvalue_10)
          (`KismetArrayLibrary.Array_Add` (`self.StaticMeshComponentArray`))
          (`StaticMeshComponent.SetStaticMesh` (`self.StaticMeshComponent`) (`self.GetMesh`))
          (`PrimitiveComponent.SetCollisionEnabled` (`self.StaticMeshComponent`) (`self.CollisionEnabled`))
          (bind _physicsmaterial_4 (`self.PhysicsMaterial`)
            (:`then`
              (`PrimitiveComponent.SetPhysMaterialOverride` (`self.StaticMeshComponent`) _physicsmaterial_4))
            (:`else`
              _))
          (`PrimitiveComponent.SetRenderCustomDepth` (`self.StaticMeshComponent`) (`self.CustomDepth`))
          (`PrimitiveComponent.SetCastShadow` (`self.StaticMeshComponent`) (`self.CastShadow`)))))))

(fn `GetLength`
  (returns (`Gap/Length` :type "Float (double-precision)"))
  (bind (_offsettransform _gaplength _usemeshlength _meshaxislength) (break `/Game/EpicMegaJam2023/Placeables/SplineTool/Structures/S_SplineTool_MainParameters` (`.MainParameters_28_05803D8A4D7C13045734EB9AF7605BC4` (break `/Game/EpicMegaJam2023/Placeables/SplineTool/Structures/S_SplineTool_ObjectList` (`self.ArrayElement`)))))
  (return (select `bool` _usemeshlength :`false` _gaplength :`true` (select `ESplineMeshAxis` _meshaxislength :`X` (.x (* (* (`.BoxExtent` (`KismetMathLibrary.BreakBoxSphereBounds` (`StaticMesh.GetBounds` (`self.GetMesh`)))) 2.0) (.scale _offsettransform))) :`Y` (.y (* (* (`.BoxExtent` (`KismetMathLibrary.BreakBoxSphereBounds` (`StaticMesh.GetBounds` (`self.GetMesh`)))) 2.0) (.scale _offsettransform))) :`Z` (.z (* (* (`.BoxExtent` (`KismetMathLibrary.BreakBoxSphereBounds` (`StaticMesh.GetBounds` (`self.GetMesh`)))) 2.0) (.scale _offsettransform)))) :!type "Float (double-precision)")))

(fn `GetMesh`
  (returns (ReturnValue :type "StaticMesh Object Reference"))
  (bind (_placementtype _staticmesh _randomsequence _mainparameters _randomparameters) (break `/Game/EpicMegaJam2023/Placeables/SplineTool/Structures/S_SplineTool_ObjectList` (`self.ArrayElement`)))
  (bind _returnvalue (- (`KismetArrayLibrary.Array_Length` _staticmesh) 1))
  (bind _returnvalue_2 (select `/Game/EpicMegaJam2023/Placeables/SplineTool/Enumerators/E_SplineToolTypes` _randomsequence :`NewEnumerator0` (`|GetArrayItem` _staticmesh) :`NewEnumerator6` (`|GetArrayItem` _staticmesh (`KismetMathLibrary.RandomIntegerInRangeFromStream` (`.RandomMeshSeed_30_8579929244985072A8DE4DB8095D2855` (break `/Game/EpicMegaJam2023/Placeables/SplineTool/Structures/S_SplineTool_Random` _randomparameters)) 0 (select `bool` (`KismetArrayLibrary.Array_IsValidIndex` _staticmesh _returnvalue) :`true` _returnvalue))) :`NewEnumerator1` (`|GetArrayItem` _staticmesh (`self.SequenceIndex`))))
  (switch `/Game/EpicMegaJam2023/Placeables/SplineTool/Enumerators/E_SplineToolTypes` _randomsequence
    (:`NewEnumerator0`
      _)
    (:`NewEnumerator6`
      _)
    (:`NewEnumerator1`
      (if (> (`self.SequenceIndex`) (`KismetArrayLibrary.Array_Length` _staticmesh))
        (set `self.SequenceIndex` 0)
        (else
          (`/Engine/EditorBlueprintResources/StandardMacros.IncrementInt` (`self.SequenceIndex`)
            (:`  `
              _))))))
  (return (select `bool` (`KismetSystemLibrary.IsValid` _returnvalue_2) :`false` (`|GetArrayItem` (`.StaticMesh_30_459BCB424BFD738D8803C588166C39B6` (break `/Game/EpicMegaJam2023/Placeables/SplineTool/Structures/S_SplineTool_ObjectList` (`self.ArrayElement`)))) :`true` _returnvalue_2)))

(fn `GetRandom`
  (returns (ReturnLocation :type "Vector Structure") (ReturnRotation :type "Rotator Structure") (ReturnScale :type "Vector Structure"))
  (bind (_placementtype _staticmesh _randomsequence _mainparameters _randomparameters) (break `/Game/EpicMegaJam2023/Placeables/SplineTool/Structures/S_SplineTool_ObjectList` (`self.ArrayElement`)))
  (bind (_randommeshseed _randomlocation _randomrotation _randomscale) (break `/Game/EpicMegaJam2023/Placeables/SplineTool/Structures/S_SplineTool_Random` _randomparameters))
  (bind (_enable _minlocationoffset _maxlocationoffset _randomlocationseed) (break `/Game/EpicMegaJam2023/Placeables/SplineTool/Structures/S_SplineTool_RandomLocationOffset` _randomlocation))
  (bind (_enable_2 _minrotationvalue _maxrotationvalue _randomrotationseed) (break `/Game/EpicMegaJam2023/Placeables/SplineTool/Structures/S_SplineTool_RandomRotationOffset` _randomrotation))
  (bind (_enable_3 _minscaevalue _maxscalevalue _randomrotationseed_2) (break `/Game/EpicMegaJam2023/Placeables/SplineTool/Structures/S_SplineTool_RandomScaleOffset` _randomscale))
  (return (select `bool` _enable :`true` (`KismetMathLibrary.MakeVector` (`KismetMathLibrary.RandomFloatInRangeFromStream` _randomlocationseed (.x _minlocationoffset) (.x _maxlocationoffset)) (`KismetMathLibrary.RandomFloatInRangeFromStream` _randomlocationseed (.y _minlocationoffset) (.y _maxlocationoffset)) (`KismetMathLibrary.RandomFloatInRangeFromStream` _randomlocationseed (.z _minlocationoffset) (.z _maxlocationoffset)))) (`KismetMathLibrary.MakeRotator` (`KismetMathLibrary.RandomFloatInRangeFromStream` _randomrotationseed (.roll _minrotationvalue) (.roll _maxrotationvalue)) (`KismetMathLibrary.RandomFloatInRangeFromStream` _randomrotationseed (.pitch _minrotationvalue) (.pitch _maxrotationvalue)) (`KismetMathLibrary.RandomFloatInRangeFromStream` _randomrotationseed (.yaw _minrotationvalue) (.yaw _maxrotationvalue))) (select `bool` _enable_3 :`false` (.scale (`.OffsetTransform_16_E65CCBA647A306B6467796A17ED42FDE` (break `/Game/EpicMegaJam2023/Placeables/SplineTool/Structures/S_SplineTool_MainParameters` _mainparameters))) :`true` (`KismetMathLibrary.MakeVector` (`KismetMathLibrary.RandomFloatInRangeFromStream` _randomrotationseed_2 (.x _minscaevalue) (.x _maxscalevalue)) (`KismetMathLibrary.RandomFloatInRangeFromStream` _randomrotationseed_2 (.y _minscaevalue) (.y _maxscalevalue)) (`KismetMathLibrary.RandomFloatInRangeFromStream` _randomrotationseed_2 (.z _minscaevalue) (.z _maxscalevalue))))))

(fn `GetScale`
  (returns (OutVector :type "Vector2D Structure"))
  (bind (_offsettransform _gaplength _usemeshlength _meshaxislength) (break `/Game/EpicMegaJam2023/Placeables/SplineTool/Structures/S_SplineTool_MainParameters` (`.MainParameters_28_05803D8A4D7C13045734EB9AF7605BC4` (break `/Game/EpicMegaJam2023/Placeables/SplineTool/Structures/S_SplineTool_ObjectList` (`self.ArrayElement`)))))
  (return (select `ESplineMeshAxis` _meshaxislength :`X` (`KismetMathLibrary.MakeVector2D` (.y (.scale _offsettransform)) (.z (.scale _offsettransform))) :`Y` (`KismetMathLibrary.MakeVector2D` (.x (.scale _offsettransform)) (.z (.scale _offsettransform))) :`Z` (`KismetMathLibrary.MakeVector2D` (.x (.scale _offsettransform)) (.y (.scale _offsettransform))))))

(fn `SetSplinePointType`)

(fn `UserConstructionScript`
  (`self.BuildSpline`))